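; Tunnel segment for an endless tunnel game, with a rotating holed wall that the player must pass through.
; RandomizeWall picks one of four hole meshes and a random roll, while Tick spins the wall and recolors tunnel and wall by player health.
; Wall overlaps damage the player or destroy projectiles.
; Reaching the trigger zone has TunnelSpawner add a segment, destroys this one, and awards score if the wall was not hit.
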(event `self.ReceiveTick`
  (params (DeltaSeconds :type "Float (single-precision)"))
  (`SceneComponent.K2_AddLocalRotation` (`self.WallMesh`) (`KismetMathLibrary.MakeRotator` (* DeltaSeconds (`self.RotateSpeed`))) false false)
  (bind _asbp_player (cast `/Game/InfiniteMatrix/Blueprints/BP_Player` (`GameplayStatics.GetPlayerPawn` 0)))
  (bind _health (`/Game/InfiniteMatrix/Blueprints/BP_Player.Health` _asbp_player))
  (if (<= _health 20.0)
    (`self.Critical Health`)
    (elif (<= _health 50.0)
      (`self.LowHealth`)
      (else
        (`PrimitiveComponent.SetMaterial` (`self.StaticMeshComponent`) 0 "/Game/InfiniteMatrix/Materials/MI_Tunnel.MI_Tunnel")
        (`PrimitiveComponent.SetMaterial` (`self.WallMesh`) 0 "/Game/InfiniteMatrix/Materials/MI_Hole.MI_Hole")))))

(event `self.TriggerZone.OnComponentBeginOverlap`
  (params (OverlappedComponent :type "PrimitiveComponent Object Reference") (OtherActor :type "Actor Object Reference") (OtherComp :type "PrimitiveComponent Object Reference") (OtherBodyIndex :type Integer) (bFromSweep :type Boolean) (SweepResult :type "HitResult Structure (by ref)"))
  (bind _asbp_player (cast `/Game/InfiniteMatrix/Blueprints/BP_Player` OtherActor))
  (`/Game/InfiniteMatrix/Blueprints/BP_TunnelSpawner.SpawnTunnelAtSpawnPoint` (`self.TunnelSpawner`))
  (`self.K2_DestroyActor`)
  (if (not (`self.HitWall`))
    (`/Game/InfiniteMatrix/Blueprints/BP_Player.IncreaseScore` _asbp_player))
  (set `self.HitWall` false))

(event `self.WallMesh.OnComponentBeginOverlap`
  (params (OverlappedComponent :type "PrimitiveComponent Object Reference") (OtherActor :type "Actor Object Reference") (OtherComp :type "PrimitiveComponent Object Reference") (OtherBodyIndex :type Integer) (bFromSweep :type Boolean) (SweepResult :type "HitResult Structure (by ref)"))
  (bind _asbp_player (cast `/Game/InfiniteMatrix/Blueprints/BP_Player` OtherActor)
    (:`then`
      (set `self.HitWall` true)
      (`/Game/InfiniteMatrix/Blueprints/BP_Player.Decrease Health` _asbp_player))
    (:`CastFailed`
      (bind _asbp_projectile (cast `/Game/InfiniteMatrix/Blueprints/BP_Projectile` OtherActor))
      (`self.K2_DestroyActor` _asbp_projectile))))

(fn `Critical Health`
  (`PrimitiveComponent.SetMaterial` (`self.StaticMeshComponent`) 0 "/Game/InfiniteMatrix/Materials/MI_TunnelRed.MI_TunnelRed")
  (`PrimitiveComponent.SetMaterial` (`self.WallMesh`) 0 "/Game/InfiniteMatrix/Materials/MI_Hole_3.MI_Hole_3"))

(fn `LowHealth`
  (`PrimitiveComponent.SetMaterial` (`self.StaticMeshComponent`) 0 "/Game/InfiniteMatrix/Materials/MI_TunnelYellow.MI_TunnelYellow")
  (`PrimitiveComponent.SetMaterial` (`self.WallMesh`) 0 "/Game/InfiniteMatrix/Materials/MI_Hole_2.MI_Hole_2"))

(fn `RandomizeWall`
  (`StaticMeshComponent.SetStaticMesh` (`self.WallMesh`) (select `int` (`KismetMathLibrary.RandomIntegerInRange` 0 3) :`0` "/Game/InfiniteMatrix/Meshes/SM_Hole_01.SM_Hole_01" :`1` "/Game/InfiniteMatrix/Meshes/SM_Hole_02.SM_Hole_02" :`2` "/Game/InfiniteMatrix/Meshes/SM_Hole_03.SM_Hole_03" :`3` "/Game/InfiniteMatrix/Meshes/SM_Hole_04.SM_Hole_04" :!type "StaticMesh Object Reference"))
  (`SceneComponent.K2_AddLocalRotation` (`self.WallMesh`) (`KismetMathLibrary.MakeRotator` (`KismetMathLibrary.RandomFloatInRange` 0.0 360.0)) false false))

(fn `UserConstructionScript`)