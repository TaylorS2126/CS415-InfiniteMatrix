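; BP_Enemy is an enemy actor that damages the player on contact and can be destroyed by projectiles for score.
; Actor overlap with BP_Player decreases its health and destroys the enemy; overlap with BP_Projectile destroys both and increases player 0's score.
; A separate TriggerZone overlap handler also destroys the enemy when the player enters, without itself changing health or score.
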(event `self.ReceiveActorBeginOverlap`
  (params (OtherActor :type "Actor Object Reference"))
  (bind _asbp_player (cast `/Game/InfiniteMatrix/Blueprints/BP_Player` OtherActor)
    (:`then`
      (`/Game/InfiniteMatrix/Blueprints/BP_Player.Decrease Health` _asbp_player)
      (`self.K2_DestroyActor`))
    (:`CastFailed`
      (bind _asbp_projectile (cast `/Game/InfiniteMatrix/Blueprints/BP_Projectile` OtherActor))
      (bind _asbp_player_2 (cast `/Game/InfiniteMatrix/Blueprints/BP_Player` (`GameplayStatics.GetPlayerPawn` 0)))
      (`self.K2_DestroyActor` _asbp_projectile)
      (`self.K2_DestroyActor`)
      (`/Game/InfiniteMatrix/Blueprints/BP_Player.IncreaseScore` _asbp_player_2))))

(event `self.TriggerZone.OnComponentBeginOverlap`
  (params (OverlappedComponent :type "PrimitiveComponent Object Reference") (OtherActor :type "Actor Object Reference") (OtherComp :type "PrimitiveComponent Object Reference") (OtherBodyIndex :type Integer) (bFromSweep :type Boolean) (SweepResult :type "HitResult Structure (by ref)"))
  (cast `/Game/InfiniteMatrix/Blueprints/BP_Player` OtherActor)
  (`/Engine/EditorBlueprintResources/StandardMacros.IsValid` self
    (:`Is Valid`
      (`self.K2_DestroyActor`))))

(fn `UserConstructionScript`)