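; BP_HealthPack is a health pickup that restores a fixed amount of the player's health, clamped to MaxHealth, and then destroys itself.
; An overlapping BP_Projectile destroys both the projectile and the pack without healing.
; A separate TriggerZone overlap also destroys the pack, without healing, when the player enters while the CurrentHealthPack reference is valid.
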(event `self.ReceiveActorBeginOverlap`
  (params (OtherActor :type "Actor Object Reference"))
  (bind _asbp_player (cast `/Game/InfiniteMatrix/Blueprints/BP_Player` OtherActor)
    (:`then`
      (set `/Game/InfiniteMatrix/Blueprints/BP_Player.Health` (`KismetMathLibrary.FClamp` (+ (`/Game/InfiniteMatrix/Blueprints/BP_Player.Health` _asbp_player) 40.0) 0.0 (`/Game/InfiniteMatrix/Blueprints/BP_Player.Max Health` _asbp_player)) _asbp_player)
      (`self.K2_DestroyActor`))
    (:`CastFailed`
      (bind _asbp_projectile (cast `/Game/InfiniteMatrix/Blueprints/BP_Projectile` OtherActor))
      (`self.K2_DestroyActor` _asbp_projectile)
      (`self.K2_DestroyActor`))))

(event `self.Trigger Zone.OnComponentBeginOverlap`
  (params (OverlappedComponent :type "PrimitiveComponent Object Reference") (OtherActor :type "Actor Object Reference") (OtherComp :type "PrimitiveComponent Object Reference") (OtherBodyIndex :type Integer) (bFromSweep :type Boolean) (SweepResult :type "HitResult Structure (by ref)"))
  (cast `/Game/InfiniteMatrix/Blueprints/BP_Player` OtherActor)
  (`/Engine/EditorBlueprintResources/StandardMacros.IsValid` (`self.CurrentHealthPack`)
    (:`Is Valid`
      (`self.K2_DestroyActor`))))

(fn `UserConstructionScript`)